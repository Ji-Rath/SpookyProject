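; BP_Television is an interactable TV that switches its audio and point light on and off.
; UpdateTV takes the state from a toggle-interactable component, both on BeginPlay and whenever that component fires OnInteract.
; It plays or stops the audio, sets the light's visibility to match, and plays a button-press cue at the actor on every update, including the initial one.
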(event OnInteract(BPC_ToggleInteractable)
  (params (Interactor :type Actor%20Object%20Reference) (Component :type Primitive%20Component%20Object%20Reference))
  (CallFunction|UpdateTV (Default|GetState (Variables|Default|GetBPC_ToggleInteractable))))

(event EventBeginPlay
  (|CallParentFunction)
  (CallFunction|UpdateTV (Default|GetState (Variables|Default|GetBPC_ToggleInteractable))))

(fn ConstructionScript)

(fn UpdateTV
  (params (bOn :type Boolean))
  (bind _audio (Variables|Default|GetAudio))
  (if bOn
    (Audio|Components|Audio|Play _audio 0.0)
    (else
      (Audio|Components|Audio|Stop _audio)))
  (Audio|PlaySoundatLocation "/Game/Assets/Sounds/ButtonPress_Cue.ButtonPress_Cue" (Transformation|GetActorLocation) "0, 0, 0" 1.0 1.0 0.0 0 0 0 0)
  (Rendering|SetVisibility (Variables|Default|GetPointLight) bOn false))
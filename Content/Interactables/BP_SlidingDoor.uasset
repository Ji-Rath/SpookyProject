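; Sliding door Blueprint that moves its Door component in a straight line according to an open percentage.
; UpdateDoorRotation, despite its name, sets relative location along the door's relative forward vector, scaled by OpenPercent and PositionDifference, with ReverseDirection flipping the sign.
; SetInitialPosition stores the actor location projected onto its forward vector as InitialPos, which neither function reads.
; Nothing in these graphs calls either function or drives OpenPercent.
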(fn ConstructionScript)

(fn UpdateDoorRotation
  (params (OpenPercent :type Float%20%28double-precision%29))
  (Transformation|SetRelativeLocation (Variables|Default|GetDoor) (* (Math|Vector|GetForwardVector (.rotation (Transformation|GetRelativeTransform (Variables|Default|GetDoor)))) (* OpenPercent (Variables|Default|GetPositionDifference) (select (Variables|Default|GetbReverseDirection) -1.0 1.0))) false false))

(fn SetInitialPosition
  (Variables|Default|SetInitialPos (Math|Vector|DotProduct (Transformation|GetActorLocation) (Math|Vector|GetForwardVector (Transformation|GetActorRotation)))))
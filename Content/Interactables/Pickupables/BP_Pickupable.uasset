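; BP_Pickupable is an interactable world item that can be picked up into an inventory.
; Its construction script synchronously loads the mesh referenced by the Item asset and applies it to the ItemMesh component.
; When InteractableComponent fires OnInteract, it adds one of that item to the interactor's InventoryComponent, then destroys itself without checking the result.
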(event OnInteract(InteractableComponent)
  (params (Interactable :type Actor%20Object%20Reference) (Interactor :type Actor%20Object%20Reference) (Component :type Scene%20Component%20Object%20Reference))
  (Class|InventoryComponent|AddtoInventory (Actor|GetComponentbyClass Interactor "/Script/InteractionSystem.InventoryComponent") (Utilities|Struct|MakeItemData (Variables|Default|GetItem) 1))
  (Actor|DestroyActor))

(event EventBeginPlay)

(event Collision|EventActorBeginOverlap
  (params (OtherActor :type Actor%20Object%20Reference)))

(event EventTick
  (params (DeltaSeconds :type Float%20%28single-precision%29)))

(fn ConstructionScript
  (bind _item (Variables|Default|GetItem)
    (:then
      (bind _returnvalue (Utilities|LoadAssetBlocking (Variables|/Script/InteractionSystem.ItemInformation|GetItemMesh _item)))
      (bind _asstatic_mesh (Utilities|Casting|CastToStaticMesh _returnvalue))
      (Components|StaticMesh|SetStaticMesh (Variables|Components|GetItemMesh) _asstatic_mesh))
    (:else)))
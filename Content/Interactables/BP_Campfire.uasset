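; Interactable campfire whose point light visibility follows the state of its toggle interactable component.
; The light syncs to that state on BeginPlay, after a SPUD save restore, and when an interaction finishes successfully.
; Using a matching item on it sets the state to off, removes the item from the user's inventory, triggers actors through the trigger component and sends an extinguished message.
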(event OnItemUse(BPC_ItemUsableComponent)
  (params (User :type Actor%20Object%20Reference) (ItemData :type Inventory%20Contents%20Structure))
  (if (Class|InventoryLibrary|IsA ItemData)
    (Class|ToggleInteractableComponent|SetState (Class|ToggleInteractable|GetToggleInteractableComponent) User false)
    (Class|InventoryComponent|RemovefromInventory (Actor|GetComponentbyClass User "/Script/InteractionSystem.InventoryComponent") (Utilities|Struct|BreakInventoryContents ItemData))
    (Class|TriggerComponent|TriggerActors (Variables|Default|GetBPC_TriggerComponent) User)
    (Class|InteractableComponent|SendInteractMessage (Class|ToggleInteractable|GetToggleInteractableComponent) User "The fire has been extinguished")))

(event OnFinishInteract(InteractableComponent)
  (params (bSuccess :type Boolean))
  (if bSuccess
    (Rendering|SetVisibility (Variables|Default|GetPointLight) (Class|ToggleInteractableComponent|GetState (Class|ToggleInteractable|GetToggleInteractableComponent)) false)))

(event EventBeginPlay
  (Rendering|SetVisibility (Variables|Default|GetPointLight) (Class|ToggleInteractableComponent|GetState (Class|ToggleInteractable|GetToggleInteractableComponent)) false))

(event EventSpudPostRestore
  (params (State :type Spud%20State%20Object%20Reference))
  (Rendering|SetVisibility (Variables|Default|GetPointLight) (Class|ToggleInteractableComponent|GetState (Class|ToggleInteractable|GetToggleInteractableComponent)) false))

(fn ConstructionScript)

(fn ShouldSkipRestoreVelocity
  (return false))

(fn ShouldSkipRestoreTransform
  (return false))

(fn GetSpudRespawnMode
  (return "Default"))
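; BP_Lightswitch is an interactable switch actor that toggles an on/off state and triggers other actors.
; Its Interactable component's OnInteract event flips IsOn, plays a button-press sound at the switch and calls TriggerActors on its TriggerComponent, with the interactor as instigator.
; Toggle and SetToggle drive the switch through that same Interact path, SetToggle only when the requested state differs from the current one.
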(event OnInteract(Interactable)
  (params (Interactable :type Actor%20Object%20Reference) (Interactor :type Actor%20Object%20Reference) (Component :type Scene%20Component%20Object%20Reference))
  (Variables|Default|SetbIsOn (not (Variables|Default|GetbIsOn)))
  (Audio|PlaySoundatLocation "/Game/Assets/Sounds/ButtonPress_Cue.ButtonPress_Cue" (Transformation|GetActorLocation) "0, 0, 0" 1.0 1.0 0.0 0 0 0 0)
  (Class|TriggerComponent|TriggerActors (Variables|Default|GetTriggerComponent) Interactor))

(event EventToggle
  (Class|InteractableComponent|Interact (Variables|Default|GetInteractable)))

(event EventSetToggle
  (params (bIsOn :type Boolean))
  (if (!= bIsOn (Variables|Default|GetbIsOn))
    (Class|InteractableComponent|Interact (Variables|Default|GetInteractable))))

(fn ConstructionScript)
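; BP_Radio is an interactable radio that plays or stops its audio when interacted with.
; On interact it reads GetState to start the Audio component from the beginning or stop it, then plays a button press sound at its location.
; The construction script sets the component's auto-activate from IsOn, so each radio can begin on or off.
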(event EventOnInteract
  (params (Interactor :type Actor%20Object%20Reference))
  (bind _audio (Variables|Default|GetAudio))
  (if (CallFunction|GetState)
    (Audio|Components|Audio|Play _audio 0.0)
    (else
      (Audio|Components|Audio|Stop _audio)))
  (Audio|PlaySoundatLocation "/Game/Assets/Sounds/ButtonPress_Cue.ButtonPress_Cue" (Transformation|GetActorLocation) "0, 0, 0" 1.0 1.0 0.0 0 0 0))

(fn ConstructionScript
  (Components|Activation|SetAutoActivate (Variables|Default|GetAudio) (Variables|Default|GetbIsOn)))
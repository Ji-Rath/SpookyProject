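; BP_Lever is an interactable physics lever that flips a toggle state as it swings between its limits.
; BeginPlay limits the physics constraint's Swing2 angle, and interaction retargets its angular orientation toward the opposite side unless RestoreState forces the negative side.
; Tick reads the current swing and updates BPCToggleInteractable once the lever nears the limit opposing the stored state, so state follows physical position rather than the interaction.
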(event OnInteract(BPC_ToggleInteractable)
  (params (Interactor :type Actor%20Object%20Reference))
  (CallFunction|SetOrientationTarget))

(event EventTick
  (params (DeltaSeconds :type Float%20%28single-precision%29))
  (if (CallFunction|IsinState)
    (Default|SetState (Variables|Default|GetBPC_ToggleInteractable) self (CallFunction|IsinonState))))

(event EventBeginPlay
  (Class|PhysicsConstraintComponent|SetAngularSwing2Limit (Variables|Default|GetPhysicsConstraint) "ACM_Limited" (Variables|Default|GetLeverLimit)))

(fn ConstructionScript)

(fn IsinState
  (bind _leverlimit (Variables|Default|GetLeverLimit))
  (return (Math|Float|NearlyEqual(Float) (Math|Float|SelectFloat _leverlimit (* -1 _leverlimit) (Default|GetState (Variables|Default|GetBPC_ToggleInteractable))) (Class|PhysicsConstraintComponent|GetCurrentSwing2 (Variables|Default|GetPhysicsConstraint)) 5.0)))

(fn IsinonState
  (return (not (Math|Float|NearlyEqual(Float) (Class|PhysicsConstraintComponent|GetCurrentSwing2 (Variables|Default|GetPhysicsConstraint)) (Variables|Default|GetLeverLimit) 5.0))))

(fn SetOrientationTarget
  (Class|PhysicsConstraintComponent|SetAngularOrientationTarget (Variables|Default|GetPhysicsConstraint) (Math|Rotator|MakeRotator 0.0 (Math|Float|SelectFloat 5e+01 -5e+01 (and (CallFunction|IsinonState) (not (Variables|Default|GetbRestoreState)))) 0.0)))
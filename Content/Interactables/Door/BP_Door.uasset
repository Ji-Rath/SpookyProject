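; Interactable hinged door that swings open and closed on a timeline driving the mesh's yaw, and can be locked behind a required key item.
; Interact and the toggle events share one open/close path.
; When locked, it compares the interactor's equipped item to the key; a match unlocks and opens it and removes that item from the inventory.
; Unlock and locked feedback go out as heads-up messages through the message subsystem.
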(event EventInteract
  (params (Interactor :type Actor%20Object%20Reference) (Component :type Scene%20Component%20Object%20Reference))
  (if (Variables|Door|GetbLocked)
    (|TryUnlockDoor Interactor Component)
    (else
      (bind _output_get (Variables|Door|SetbIsOn (not (Variables|Door|GetbIsOn))))
      (if _output_get
        (bind _newtrack_0 (Timeline|OpenDoor Play)
          (:Update
            (Transformation|SetRelativeRotation (Variables|Default|GetDoorMesh) (Math|Rotator|MakeRotator 0.0 0.0 (* _newtrack_0 9e+01)) false false)))
        (else
          (Timeline|OpenDoor Reverse))))))

(event EventToggle
  (Class|Interactable|Interact))

(event EventSetToggle
  (params (bIsOn :type Boolean))
  (if (!= bIsOn (Variables|Door|GetbIsOn))
    (Class|Interactable|Interact)))

(fn ConstructionScript)

(fn CanUnlockDoor
  (params (Item :type Item%20Information%20Object%20Reference))
  (return (== Item (Variables|Door|GetKeyRequired))))

(fn CanInteract
  (params (Interactor :type Actor%20Object%20Reference) (Component :type Scene%20Component%20Object%20Reference))
  (return true))

(fn GetInteractType
  (return "SingleUse"))

(fn GetName
  (params (Component :type Scene%20Component%20Object%20Reference))
  (return ""))
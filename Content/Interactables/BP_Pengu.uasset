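; Pengu is an interactable NPC and dialogue participant tied to the escape-house quest.
; Interacting with a hammer equipped spawns a key pickup once and fires OnDropKey; otherwise it opens D_Pengu in a dialogue widget on the HUD's full-screen stack.
; Dialogue conditions match the current Q_EscapeHouse objective identifier, and the "Give Key" dialogue event actually spawns a hammer head pickup, with no repeat guard.
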(event OnInteract(Interactable)
  (params (Interactable :type Actor%20Object%20Reference) (Interactor :type Actor%20Object%20Reference) (Component :type Scene%20Component%20Object%20Reference))
  (if (CallFunction|HasItemEquipped Interactor "/Game/Interactables/Pickupables/DA_Hammer.DA_Hammer")
    (if (not (Variables|Default|GetbGaveKey))
      (Game|SpawnActorfromClass "/Game/Interactables/Pickupables/BP_Pickupable.BP_Pickupable_C" (Math|Conversions|ToTransform(Vector) (Transformation|GetActorLocation)) "AdjustIfPossibleButAlwaysSpawn" "MultiplyWithRoot" 0 "/Game/Interactables/Pickupables/DA_Key.DA_Key" 0)
      (Variables|Default|SetbGaveKey true)
      (Default|CallOnDropKey))
    (else
      (bind _returnvalue (Class|DlgManager|StartDialogue "/Game/Dialogue/D_Pengu.D_Pengu" (Utilities|Array|MakeArray self)))
      (bind _widget (Class|IBaseCanvasHolder|GetBaseCanvas(Message) (HUD|GetHUD (Game|GetPlayerController 0))))
      (bind _returnvalue_2 (Class|CommonActivatableWidgetContainerBase|AddWidget (Variables|/Game/UI/WBP_BaseCanvas.WBP_BaseCanvas_C|GetFullScreenStack _widget) "/Game/UI/Dialogue/WBP_Dialogue.WBP_Dialogue_C"))
      (Default|SetDialogue _returnvalue_2 _returnvalue))))

(fn ConstructionScript)

(fn CheckCondition
  (params (Context :type Dlg%20Context%20Object%20Reference) (ConditionName :type Name :default "None"))
  (bind _progression (Class|IQuestManager|GetCurrentProgression(Message) (Game|GetGameState)))
  (Utilities|IsValid (Class|SuqsProgression|GetCurrentObjective _progression "Q_EscapeHouse")
    (:Is%20Valid
      (return (== (Class|SuqsObjectiveState|GetIdentifier (Class|SuqsProgression|GetCurrentObjective _progression "Q_EscapeHouse")) ConditionName)))
    (:Is%20Not%20Valid
      (return false))))

(fn GetBoolValue
  (params (ValueName :type Name :default "None"))
  (return false))

(fn GetFloatValue
  (params (ValueName :type Name :default "None"))
  (return 0.0))

(fn GetIntValue
  (params (ValueName :type Name :default "None"))
  (return 0))

(fn GetNameValue
  (params (ValueName :type Name :default "None"))
  (return "None"))

(fn GetParticipantDisplayName
  (params (ActiveSpeaker :type Name :default "None"))
  (return "Pengu"))

(fn GetParticipantGender
  (return "Masculine"))

(fn GetParticipantIcon
  (params (ActiveSpeaker :type Name :default "None") (ActiveSpeakerState :type Name :default "None"))
  (return 0))

(fn GetParticipantName
  (return "Pengu"))

(fn ModifyBoolValue
  (params (ValueName :type Name :default "None") (bNewValue :type Boolean))
  (return false))

(fn ModifyFloatValue
  (params (ValueName :type Name :default "None") (bDelta :type Boolean) (Value :type Float%20%28single-precision%29))
  (return false))

(fn ModifyIntValue
  (params (ValueName :type Name :default "None") (bDelta :type Boolean) (Value :type Integer))
  (return false))

(fn ModifyNameValue
  (params (ValueName :type Name :default "None") (NameValue :type Name :default "None"))
  (return false))

(fn OnDialogueEvent
  (params (Context :type Dlg%20Context%20Object%20Reference) (EventName :type Name :default "None"))
  (|SwitchDialogueCallbackEvent EventName
    (:GiveKey
      (Game|SpawnActorfromClass "/Game/Interactables/Pickupables/BP_Pickupable.BP_Pickupable_C" (Math|Conversions|ToTransform(Vector) (Transformation|GetActorLocation)) "AdjustIfPossibleButAlwaysSpawn" "MultiplyWithRoot" 0 "/Game/Interactables/Pickupables/DA_HammerHead.DA_HammerHead" 0)
      (return true))))
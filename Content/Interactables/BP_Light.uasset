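; BP_Light is an interactable point light that players toggle off and on.
; Each OnInteract call flips between saving the attenuation radius then setting it to zero, and restoring the saved radius.
; When Flicker is enabled, the construction script applies a dynamic M_LightFlicker light function material with a random Offset, so each instance gets its own flicker offset.
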(event OnInteract(Interactable)
  (params (Interactable :type Actor%20Object%20Reference) (Interactor :type Actor%20Object%20Reference) (Component :type Scene%20Component%20Object%20Reference))
  (Utilities|FlowControl|FlipFlop
    (:A
      (Variables|Default|SetOldLightRadius (Variables|/Script/Engine.LocalLightComponent|GetAttenuationRadius (Variables|Default|GetPointLight)))
      (Rendering|Lighting|SetAttenuationRadius (Variables|Default|GetPointLight) 0.0))
    (:B
      (Rendering|Lighting|SetAttenuationRadius (Variables|Default|GetPointLight) (Variables|Default|GetOldLightRadius)))))

(event EventBeginPlay)

(event Collision|EventActorBeginOverlap
  (params (OtherActor :type Actor%20Object%20Reference)))

(event EventTick
  (params (DeltaSeconds :type Float%20%28single-precision%29)))

(fn ConstructionScript
  (if (Variables|Default|GetbFlicker)
    (bind _returnvalue (Rendering|Material|CreateDynamicMaterialInstance "/Game/Assets/M_LightFlicker.M_LightFlicker" "None" "None" :!class /Script/Engine.KismetMaterialLibrary))
    (Rendering|Components|Light|SetLightFunctionMaterial (Variables|Default|GetPointLight) _returnvalue)
    (Rendering|Material|SetScalarParameterValue _returnvalue "Offset" (Math|Random|RandomFloatinRange -1e+02 1e+02) :!class /Script/Engine.MaterialInstanceDynamic)))
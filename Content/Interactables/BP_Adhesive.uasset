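; BP_Adhesive is a single-use interactable that lets the player collect adhesive with a spoon.
; On interact, it checks the equipped item: a spoon is swapped in the inventory for a spoon-with-adhesive item, and the actor destroys itself.
; Collection or a wrong item sends a heads-up through the message subsystem, while no valid equipped item data produces no response.
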(event Custom|Interact_1_1
  (params (Interactor :type Actor%20Object%20Reference) (Component :type Scene%20Component%20Object%20Reference))
  (bind _returnvalue (Actor|GetComponentbyClass Interactor "/Script/InteractionSystem.InventoryComponent"))
  (bind _value (Utilities|InstancedStruct|GetInstancedStructValue (Utilities|Struct|BreakInventoryContents (CallFunction|TryGetEquippedItemData Interactor)))
    (:Valid
      (if (== (Utilities|Struct|BreakItemData _value) "/Game/Interactables/Pickupables/DA_Spoon.DA_Spoon")
        (Class|InventoryComponent|AddtoInventory _returnvalue (Utilities|Struct|MakeItemData "/Game/Interactables/Pickupables/DA_SpoonAdhesive.DA_SpoonAdhesive" 1))
        (Class|InventoryComponent|RemovefromInventory _returnvalue (Class|PlayerEquipComponent|GetEquippedItem (Actor|GetComponentbyClass Interactor "/Script/InteractionSystem.PlayerEquipComponent")))
        (bind _returnvalue_2 (Utilities|InstancedStruct|MakeInstancedStruct (Variables|Default|GetCollectAdhesiveMessage)))
        (Class|MessageSubsystem|SendMessage (Subsystems|GetMessageSubsystem) "(TagName=\"Message.HeadsUp\")" _returnvalue_2)
        (Actor|DestroyActor)
        (else
          (bind _returnvalue_3 (Utilities|InstancedStruct|MakeInstancedStruct (Variables|Default|GetNoSpoonMessage)))
          (Class|MessageSubsystem|SendMessage (Subsystems|GetMessageSubsystem) "(TagName=\"Message.HeadsUp\")" _returnvalue_3))))))

(event EventBeginPlay)

(event Collision|EventActorBeginOverlap
  (params (OtherActor :type Actor%20Object%20Reference)))

(event EventTick
  (params (DeltaSeconds :type Float%20%28single-precision%29)))

(fn ConstructionScript)

(fn CanInteract
  (params (Interactor :type Actor%20Object%20Reference) (Component :type Scene%20Component%20Object%20Reference))
  (return true))

(fn GetInteractType
  (return "SingleUse"))

(fn GetName
  (params (Component :type Scene%20Component%20Object%20Reference))
  (return ""))
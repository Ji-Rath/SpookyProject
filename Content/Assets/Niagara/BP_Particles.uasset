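; BP_Particles is a Niagara particle actor whose effect tracks the location of a referenced light actor.
; UpdateFollowPos writes that actor's location into the Niagara LightPos variable, both during construction and every Tick.
; The construction script also passes a Direction float to the Niagara component once, so it does not update at runtime.
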(event EventTick
  (params (DeltaSeconds :type Float%20%28single-precision%29))
  (CallFunction|UpdateFollowPos))

(fn ConstructionScript
  (CallFunction|UpdateFollowPos)
  (Niagara|SetNiagaraVariable(Float) (Variables|Default|GetNiagaraComponent0) "Direction" (Variables|Default|GetDirection)))

(fn UpdateFollowPos
  (Niagara|SetNiagaraVariable(Vector3) (Variables|Default|GetNiagaraComponent0) "LightPos" (Transformation|GetActorLocation (Variables|Default|GetLightActor))))
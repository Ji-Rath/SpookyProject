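; BP_AdditionalAction is an interactable helper that applies configured side effects to other objects when its OnTrigger event fires.
; It optionally plays a sound at its location, then sets the interaction and player-interaction flags on each SetInteractable entry.
; It then sets the Locked state on BP_Door references in SetLockStatus.
; SetOn loops over the same lock array without doing anything and is not called here.
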(event EventOnTrigger
  (CallFunction|PlaySound)
  (CallFunction|MakeInteractable)
  (CallFunction|SetLock))

(fn ConstructionScript)

(fn PlaySound
  (if (Variables|Actions|GetbPlaySound)
    (Audio|PlaySoundatLocation (Variables|Actions|GetSound) (Transformation|GetActorLocation) "0, 0, 0" 1.0 1.0 0.0 0 0 0)))

(fn MakeInteractable
  (for _array_element (Variables|Actions|GetSetInteractable)
    (Variables|/Script/SpookyGame.InteractableBase|SetbCanInteract (.InteractableRef (Utilities|Struct|BreakMakeInteractableStruct _array_element)) (.MakeInteractable (Utilities|Struct|BreakMakeInteractableStruct _array_element)))
    (Variables|/Script/SpookyGame.InteractableBase|SetbPlayerInteract (.InteractableRef (Utilities|Struct|BreakMakeInteractableStruct _array_element)) (.MakePlayerInteractable (Utilities|Struct|BreakMakeInteractableStruct _array_element)))))

(fn SetLock
  (for _array_element (Variables|Actions|GetSetLockStatus)
    (bind _asbp_door (Utilities|Casting|CastToBP_Door (.interactableref _array_element)))
    (Variables|/Game/Blueprints/Interactables/BP_Door.BP_Door_C|SetbLocked _asbp_door (.bison _array_element))))

(fn Seton
  (for _array_element (Variables|Actions|GetSetLockStatus)
    _))
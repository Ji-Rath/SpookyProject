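; An interactable television that the player switches on and off, with looping or one-shot audio and a screen light.
; Construction sets the point light visibility from IsOn, and BeginPlay stops the audio when the set starts off.
; Each interaction flips IsOn, starts or stops the audio, toggles the light, and plays a button press sound at the actor's location.
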(event EventOnInteract
  (params (Interactor :type Actor%20Object%20Reference))
  (bind _audio (Variables|Default|GetAudio))
  (bind _output_get (Variables|Default|SetbIsOn (not (Variables|Default|GetbIsOn))))
  (if _output_get
    (Audio|Components|Audio|Play _audio 0.0)
    (else
      (Audio|Components|Audio|Stop _audio)))
  (Audio|PlaySoundatLocation "/Game/Assets/Sounds/ButtonPress_Cue.ButtonPress_Cue" (Transformation|GetActorLocation) "0, 0, 0" 1.0 1.0 0.0 0 0 0)
  (Rendering|ToggleVisibility (Variables|Default|GetPointLight) false))

(event EventBeginPlay
  (|CallParentFunction)
  (if (not (Variables|Default|GetbIsOn))
    (Audio|Components|Audio|Stop (Variables|Default|GetAudio))))

(fn ConstructionScript
  (Rendering|SetVisibility (Variables|Default|GetPointLight) (Variables|Default|GetbIsOn) false))
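; An interactable door that swings open and closed on yaw via a timeline, with sounds, and plays a jam animation when locked.
; Using the matching key item on a locked door drops it from the player's hand and binds it and the door into an unlock level sequence anchored to the door's transform.
; Interaction is blocked while unlocking; OpenDoor clears the lock, opens the door and returns the key to the inventory.
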(event Custom|UnlockSequence
  (params (Item :type Item%20Data%20Object%20Reference) (User :type Actor%20Object%20Reference))
  (CallFunction|UnlockDoor Item User))

(event Custom|OpenDoor
  (Variables|DoorPosition|SetbLocked false)
  (Variables|Default|SetbUnlockingDoor false)
  (Class|Interactable|Interact (stale Custom|UnlockSequence User))
  (CallFunction|GiveItem (stale Custom|UnlockSequence User)))

(event Custom|DoorJam
  (Audio|PlaySoundatLocation (Variables|DoorSounds|GetDoorLocked) (Transformation|GetWorldLocation (Variables|Default|GetSoundLocation)) "0, 0, 0" 1.0 1.0 0.0 0 0 0)
  (bind _newtrack_0 (Timeline|DoorJammed PlayFromStart)
    (:Update
      (CallFunction|UpdateDoorRotation _newtrack_0))))

(event EventOnInteract
  (params (Interactor :type Actor%20Object%20Reference))
  (if (CallFunction|CanInteract Interactor)
    (if (Variables|DoorPosition|GetbLocked)
      (CallFunction|DoorJam)
      (else
        (bind _isa (Utilities|FlowControl|FlipFlop) ; Flip between open/closed door
          (:A
            (Audio|PlaySoundatLocation (Variables|DoorSounds|GetDoorOpen) (Transformation|GetWorldLocation (Variables|Default|GetSoundLocation)) "0, 0, 0" 1.0 1.0 0.0 0 0 0)
            (bind _newtrack_0 (Timeline|DoorOpen/Close Play)
              (:Update
                (CallFunction|UpdateDoorRotation _newtrack_0))
              (:Finished
                (if (not _isa)
                  (Audio|PlaySoundatLocation (Variables|DoorSounds|GetDoorClose) (Transformation|GetWorldLocation (Variables|Default|GetSoundLocation)) "0, 0, 0" 1.0 1.0 0.0 0 0 0)))))
          (:B
            (Timeline|DoorOpen/Close Reverse)))))))

(fn ConstructionScript
  (CallFunction|SetInitialPosition))

(fn UpdateDoorRotation
  (params (OpenPercent :type Float%20%28single-precision%29))
  (bind _returnvalue (Transformation|GetActorRotation))
  (Transformation|SetActorRotation (Math|Rotator|MakeRotator (.roll _returnvalue) (.pitch _returnvalue) (+ (* OpenPercent (Variables|DoorPosition|GetPositionDifference) (Math|Float|SelectFloat -1.0 1.0 (Variables|DoorPosition|GetbReverseDirection))) (Variables|DoorPosition|GetInitialPos)))))

(fn SetInitialPosition
  (Variables|DoorPosition|SetInitialPos (.yaw (Transformation|GetActorRotation))))

(fn CanUnlockDoor
  (params (Item :type Item%20Data%20Object%20Reference))
  (if (and (Utilities|IsValid Item) (Utilities|IsValid (Variables|DoorUnlock|GetDoorKey))) ; Ensure tested keys are valid
    (return (== Item (Variables|DoorUnlock|GetDoorKey)))))

(fn UnlockDoor
  (params (ItemData :type Item%20Data%20Object%20Reference) (User :type Actor%20Object%20Reference))
  (if (not (Variables|Default|GetbUnlockingDoor))
    (CallFunction|TakeItem User)
    (bind (_outactor _returnvalue) (Sequencer|Player|CreateLevelSequencePlayer (Variables|DoorUnlock|GetDoorUnlockSequence) (Variables|Default|GetSequenceSettings)))
    (CallFunction|SetLevelSequenceOrigin _outactor (Transformation|GetActorTransform))
    (Class|LevelSequenceActor|AddBinding _outactor (|GetSequenceBinding) self false)
    (Class|LevelSequenceActor|AddBinding _outactor (|GetSequenceBinding) (Variables|Default|GetKeyReference) false)
    (EventDispatchers|BindEventtoOnFinished _returnvalue (EventDispatchers|CreateEvent :!event Custom|OpenDoor))
    (Variables|Default|SetbUnlockingDoor true)))

(fn CanInteract
  (params (Interactor :type Actor%20Object%20Reference))
  (return (and (|CallParentFunction Interactor) (not (Variables|Default|GetbUnlockingDoor)))))

(fn SetLevelSequenceOrigin
  (params (LevelSequence :type Level%20Sequence%20Actor%20Object%20Reference) (TransformOrigin :type Transform))
  (Variables|/Script/LevelSequence.LevelSequenceActor|SetbOverrideInstanceData LevelSequence true)
  (bind _asdefault_level_sequence_instance_data (Utilities|Casting|CastToDefaultLevelSequenceInstanceData (Variables|/Script/LevelSequence.LevelSequenceActor|GetDefaultInstanceData LevelSequence)))
  (Variables|/Script/LevelSequence.DefaultLevelSequenceInstanceData|SetTransformOrigin _asdefault_level_sequence_instance_data TransformOrigin))

(fn TakeItem
  (params (Interactor :type Actor%20Object%20Reference))
  (bind _returnvalue (Actor|GetComponentbyClass Interactor "/Script/InteractionSystem.PlayerEquipComponent"))
  (Variables|Default|SetKeyReference (Class|PlayerEquipComponent|GetEquippedItem _returnvalue))
  (Class|PlayerEquipComponent|DropEquippedItem _returnvalue))

(fn GiveItem
  (params (User :type Actor%20Object%20Reference))
  (bind _keyreference (Variables|Default|GetKeyReference))
  (Class|InventoryComponent|AddtoInventory (Actor|GetComponentbyClass User "/Game/Blueprints/Components/BP_Inventory.BP_Inventory_C") (Class|Pickupable|GetItemData _keyreference) 1)
  (Actor|DestroyActor _keyreference))

(fn OnItemUse
  (params (User :type Actor%20Object%20Reference) (Item :type Item%20Data%20Object%20Reference))
  (if (Variables|DoorPosition|GetbLocked)
    (Utilities|IsValid (Variables|DoorUnlock|GetDoorKey) ; Attempt to unlock door if possible
      (:Is%20Valid
        (if (CallFunction|CanUnlockDoor Item)
          (CallFunction|UnlockSequence Item User)
          (return true)
          (else
            (CallFunction|DoorJam)
            (return false))))
      (:Is%20Not%20Valid
        (CallFunction|DoorJam)))
    (else
      (return false))))
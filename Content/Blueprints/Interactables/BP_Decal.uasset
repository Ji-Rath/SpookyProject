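; BP_Decal is an interactable decal actor that plays an animated flipbook through its decal material.
; On begin play it creates a dynamic material instance and derives the last frame from the material's Columns and Rows parameters.
; A looping timer increments the Frame parameter while the decal is visible, wrapping at the end and hiding the decal if looping is off.
; OnTrigger toggles the decal's visibility and restarts the animation.
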(event EventOnTrigger
  (Rendering|ToggleVisibility (Variables|Default|GetNewDecalComponent) false)
  (Variables|Default|SetFrame 0.0))

(event EventBeginPlay
  (bind _returnvalue (Rendering|Material|CreateDynamicMaterialInstance (Variables|Default|GetNewDecalComponent) :!class /Script/Engine.DecalComponent))
  (bind _output_get (Variables|Default|SetMaterialInstance _returnvalue))
  (bind _returnvalue_2 (Rendering|Material|GetScalarParameterValue _output_get "Columns" :!class /Script/Engine.MaterialInstanceDynamic))
  (bind _returnvalue_3 (Rendering|Material|GetScalarParameterValue _output_get "Rows" :!class /Script/Engine.MaterialInstanceDynamic))
  (Variables|Default|SetLastFrame (- (* _returnvalue_3 _returnvalue_2) 1.0))
  (Utilities|Time|SetTimerbyFunctionName 0 "IncrementFrame" (Variables|Default|GetAnimationSpeed) true))

(fn ConstructionScript)

(fn IncrementFrame
  (if (Rendering|IsVisible (Variables|Default|GetNewDecalComponent))
    (bind _result (Math|Float|IncrementFloat (Variables|Default|GetFrame))
      (:%20%20
        (Rendering|Material|SetScalarParameterValue (Variables|Default|GetMaterialInstance) "Frame" _result :!class /Script/Engine.MaterialInstanceDynamic)
        (if (> (Variables|Default|GetFrame) (Variables|Default|GetLastFrame))
          (if (not (Variables|Default|GetbAnimationLoop))
            (Rendering|ToggleVisibility (Variables|Default|GetNewDecalComponent) false))
          (Variables|Default|SetFrame 0.0))))))
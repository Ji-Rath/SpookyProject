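; Sliding door interactable that moves the whole actor in a straight line according to an open percentage.
; BeginPlay runs the parent logic, then caches the starting world X position.
; UpdateDoorRotation, despite its name, offsets location by the forward vector scaled by OpenPercent and PositionDifference, with an optional direction flip.
; Only the X component is applied, so the door slides solely along world X, keeping its current Y and Z.
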(event EventBeginPlay
  (|CallParentFunction)
  (Variables|Default|SetInitialPos (.x (Transformation|GetActorLocation))))

(fn ConstructionScript)

(fn UpdateDoorRotation
  (params (OpenPercent :type Float%20%28single-precision%29))
  (bind _returnvalue (Transformation|GetActorLocation))
  (Transformation|SetActorLocation (Math|Vector|MakeVector (+ (.x (* (Math|Vector|GetForwardVector (Transformation|GetActorRotation)) (* OpenPercent (Variables|Default|GetPositionDifference) (select (Variables|Default|GetbReverseDirection) -1.0 1.0)))) (Variables|Default|GetInitialPos)) (.y _returnvalue) (.z _returnvalue)) false false))
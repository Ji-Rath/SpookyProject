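; BP_Radio is an interactable radio that the player switches on and off.
; Each interaction flips IsOn, plays or stops the Audio component from the start, and plays a button press cue at the actor's location.
; The construction script sets the Audio component's auto-activate from IsOn, so a placed radio can start already playing.
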(event EventOnInteract
  (params (Interactor :type Actor%20Object%20Reference))
  (bind _audio (Variables|Default|GetAudio))
  (bind _output_get (Variables|Default|SetbIsOn (not (Variables|Default|GetbIsOn))))
  (if _output_get
    (Audio|Components|Audio|Play _audio 0.0)
    (else
      (Audio|Components|Audio|Stop _audio)))
  (Audio|PlaySoundatLocation "/Game/Assets/Sounds/ButtonPress_Cue.ButtonPress_Cue" (Transformation|GetActorLocation) "0, 0, 0" 1.0 1.0 0.0 0 0 0))

(fn ConstructionScript
  (Components|Activation|SetAutoActivate (Variables|Default|GetAudio) (Variables|Default|GetbIsOn)))
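; BP_DoorLatch is a door latch actor that rotates about its roll axis according to a door's open percentage.
; SetInitialPosition caches the starting roll as InitialPos.
; UpdateDoorRotation scales the open percentage by PositionDifference, flips the sign when ReverseDirection is set, and adds InitialPos, preserving pitch and yaw.
; Its construction script only runs the parent's, and the file shows no caller for either function.
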(fn ConstructionScript
  (|CallParentFunction))

(fn UpdateDoorRotation
  (params (OpenPercent :type Float%20%28single-precision%29))
  (bind _returnvalue (Transformation|GetActorRotation))
  (Transformation|SetActorRotation (Math|Rotator|MakeRotator (+ (* OpenPercent (Variables|Default|GetPositionDifference) (Math|Float|SelectFloat -1.0 1.0 (Variables|Default|GetbReverseDirection))) (Variables|Default|GetInitialPos)) (.pitch _returnvalue) (.yaw _returnvalue))))

(fn SetInitialPosition
  (Variables|Default|SetInitialPos (.roll (Transformation|GetActorRotation))))
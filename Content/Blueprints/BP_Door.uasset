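; BP_Door is a swinging door that opens and closes on alternate OnTrigger calls, or plays a locked reaction when Locked.
; Timelines drive actor yaw relative to the rotation captured at BeginPlay, scaled by 90 degrees.
; A FlipFlop plays or reverses the open/close timeline, with sounds at opening start and once closing finishes.
; When locked, a separate timeline animates the yaw alongside a locked sound.
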(event EventOnTrigger
  (bind _soundlocation (Variables|Default|GetSoundLocation))
  (bind _returnvalue (Transformation|GetWorldLocation _soundlocation))
  (if (Variables|Default|GetbLocked)
    (Audio|PlaySoundatLocation "/Game/Assets/Sounds/DoorLocked_Cue.DoorLocked_Cue" _returnvalue "0, 0, 0" 1.0 1.0 0.0 0 0 0)
    (bind _newtrack_0 (Timeline|DoorLocked PlayFromStart)
      (:Update
        (Transformation|SetActorRotation (Math|Rotator|MakeRotator 0.0 0.0 (+ (* _newtrack_0 9e+01) (Variables|Default|GetInitialYaw))))))
    (else
      (bind _isa (Utilities|FlowControl|FlipFlop)
        (:A
          (Audio|PlaySoundatLocation "/Game/Assets/Sounds/DoorOpen_Cue.DoorOpen_Cue" _returnvalue "0, 0, 0" 1.0 1.0 0.0 0 0 0)
          (bind _newtrack_0_2 (Timeline|DoorOpen/Close Play)
            (:Update
              (Transformation|SetActorRotation (Math|Rotator|MakeRotator 0.0 0.0 (+ (* _newtrack_0_2 9e+01) (Variables|Default|GetInitialYaw)))))
            (:Finished
              (if (not _isa)
                (Audio|PlaySoundatLocation "/Game/Assets/Sounds/DoorClose_Cue.DoorClose_Cue" _returnvalue "0, 0, 0" 1.0 1.0 0.0 0 0 0)))))
        (:B
          (Timeline|DoorOpen/Close Reverse))))))

(event EventBeginPlay
  (Variables|Default|SetInitialYaw (.yaw (Transformation|GetActorRotation))))

(fn ConstructionScript)
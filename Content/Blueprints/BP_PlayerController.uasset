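; Player controller that manages title and in-game UI states and swaps control between an awake player pawn and a sleeping one.
; On BeginPlay it caches the BP_Player and BP_PlayerSleeping actors, then shows the title widget with UI-only input and a cursor.
; MainGame swaps in the main HUD, sets the view target to the controlled pawn and restores game-only input.
; BlinkAction unpossesses and uses a FlipFlop to alternate possession between the two pawns.
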(event EventBeginPlay
  (CallFunction|GetPlayerRef)
  (CallFunction|TitleScreen))

(event EventBlinkAction
  (Pawn|UnPossess)
  (Utilities|FlowControl|FlipFlop
    (:A
      (Pawn|Possess (Variables|Default|GetPlayerRef)))
    (:B
      (Pawn|Possess (Variables|Default|GetSleepingPawn)))))

(fn ConstructionScript)

(fn TitleScreen
  (Viewport|RemoveAllWidgets)
  (bind _returnvalue (UserInterface|CreateWidget "/Game/Blueprints/Widgets/Widget_Title.Widget_Title_C"))
  (UserInterface|Viewport|AddtoViewport _returnvalue 0)
  (Input|SetInputModeUIOnly self _returnvalue "DoNotLock")
  (Variables|Default|SetbShowMouseCursor true))

(fn MainGame
  (Viewport|RemoveAllWidgets)
  (bind _returnvalue (UserInterface|CreateWidget "/Game/Blueprints/Widgets/Widget_MainUI.Widget_MainUI_C"))
  (UserInterface|Viewport|AddtoViewport _returnvalue 0)
  (Variables|Default|SetMainUI _returnvalue)
  (Game|Player|SetViewTargetwithBlend (Game|GetPlayerController 0) (Pawn|GetControlledPawn) 0.0 "VTBlend_Linear" 0.0 false)
  (Input|SetInputModeGameOnly self)
  (Variables|Default|SetbShowMouseCursor false))

(fn GetPlayerRef
  (bind _returnvalue (Actor|GetActorOfClass "/Game/Blueprints/BP_Player.BP_Player_C"))
  (Variables|Default|SetPlayerRef _returnvalue)
  (bind _returnvalue_2 (Actor|GetActorOfClass "/Game/Blueprints/BP_PlayerSleeping.BP_PlayerSleeping_C"))
  (Variables|Default|SetSleepingPawn _returnvalue_2))
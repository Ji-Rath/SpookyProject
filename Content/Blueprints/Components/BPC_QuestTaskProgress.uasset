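; Actor component that advances or completes a quest task, intended for owners that implement or derive from Interactable.
; On BeginPlay it casts its owner to Interactable and binds an event to its OnInteracted.
; TriggerQuestTask reaches the SUQS progression on GS_SpookyGame, then either completes the configured task or progresses it by Delta, depending on the CompleteTask flag.
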(event EventBeginPlay
  (bind _asinteractable (Utilities|Casting|CastToInteractable (Components|GetOwner)))
  (EventDispatchers|BindEventtoOnInteracted _asinteractable (EventDispatchers|CreateEvent :!event TriggerQuestTask)))

(fn TriggerQuestTask
  (params (Interactor :type Actor%20Object%20Reference))
  (bind _asgs_spooky_game (Utilities|Casting|CastToGS_SpookyGame (Game|GetGameState)))
  (if (Variables|Task|GetbCompleteTask)
    (Class|SuqsProgression|CompleteTask (Variables|/Game/Blueprints/GS_SpookyGame.GS_SpookyGame_C|GetSUQS_Progression _asgs_spooky_game) (Variables|Task|GetQuestID) (Variables|Task|GetQuestTask))
    (else
      (Class|SuqsProgression|ProgressTask (Variables|/Game/Blueprints/GS_SpookyGame.GS_SpookyGame_C|GetSUQS_Progression _asgs_spooky_game) (Variables|Task|GetQuestID) (Variables|Task|GetQuestTask) (Variables|Task|TaskProgress|GetDelta)))))
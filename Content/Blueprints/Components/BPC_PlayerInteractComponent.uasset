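; BPC_PlayerInteractComponent is a player component that forwards interact and item-use actions to a target actor.
; ComponentInteract looks up the target's BPC_Interactable and calls its interact handler with the owner as instigator.
; ComponentItemUse passes the owner and the equipped item data from its PlayerEquipComponent to the target's BPC_ItemUsableComponent.
; Both rely on component lookup with validity checks, so targets lacking the matching component are ignored.
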(fn ComponentInteract
  (params (Interactable :type Actor%20Object%20Reference))
  (bind _returnvalue (Actor|GetComponentbyClass Interactable "/Game/Blueprints/Components/BPC_Interactable.BPC_Interactable_C"))
  (Utilities|IsValid _returnvalue
    (:Is%20Valid
      (Default|CallOnInteract _returnvalue (Components|GetOwner)))))

(fn ComponentItemUse
  (params (Interactable :type Actor%20Object%20Reference))
  (bind _returnvalue (Actor|GetComponentbyClass Interactable "/Game/Blueprints/Components/BPC_ItemUsableComponent.BPC_ItemUsableComponent_C"))
  (bind _returnvalue_2 (Components|GetOwner))
  (bind _returnvalue_3 (Actor|GetComponentbyClass _returnvalue_2 "/Script/InteractionSystem.PlayerEquipComponent"))
  (if (and (Utilities|IsValid _returnvalue) (Utilities|IsValid _returnvalue_3))
    (Default|CallOnItemUse _returnvalue (Components|GetOwner) (Class|PlayerEquipComponent|GetEquippedItemData _returnvalue_3))))
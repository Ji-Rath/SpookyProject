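; BPC_LevelLoad is an actor component that swaps streamed levels when its owner is interacted with.
; On BeginPlay it binds two events to the owner's InteractableComponent OnInteract dispatcher.
; One event unloads LevelUnload and the other loads LevelLoad as visible, kept separate because both stream asynchronously without blocking.
; The load event then broadcasts OnLoadLevel.
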(event Custom|UnloadStreamLevel
  (params (Interactor :type Actor%20Object%20Reference) (Component :type Primitive%20Component%20Object%20Reference))
  (Class|GameplayStatics|UnloadStreamLevelbySoftObjectPtr (Variables|Default|GetLevelUnload) false))

(event Custom|LoadStreamLevel
  (params (Interactor :type Actor%20Object%20Reference) (Component :type Primitive%20Component%20Object%20Reference))
  (Class|GameplayStatics|LoadStreamLevelbySoftObjectPtr (Variables|Default|GetLevelLoad) true false)
  (Default|CallOnLoadLevel))

(event EventBeginPlay
  (bind _returnvalue (Components|GetOwner))
  (bind _returnvalue_2 (Actor|GetComponentbyClass _returnvalue "/Script/InteractionSystem.InteractableComponent"))
  (EventDispatchers|BindEventtoOnInteract _returnvalue_2 (EventDispatchers|CreateEvent :!event Custom|UnloadStreamLevel))
  (EventDispatchers|BindEventtoOnInteract _returnvalue_2 (EventDispatchers|CreateEvent :!event Custom|LoadStreamLevel)))
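; Player controller that runs the main game UI and switches control between the awake player and a sleeping player pawn.
; BeginPlay caches both pawns by class lookup, then MainGame swaps in the main UI widget, sets the view target and mouse state.
; BlinkAction unpossesses, then uses a FlipFlop to alternately possess each pawn, starting with BP_Player.
; A TitleScreen function builds the title widget, but its call in the event graph is unconnected.
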(event EventBeginPlay
  (CallFunction|GetPlayerRef)
  (CallFunction|MainGame))

(event EventBlinkAction
  (Pawn|UnPossess)
  (Utilities|FlowControl|FlipFlop
    (:A
      (Pawn|Possess (Variables|Default|GetPlayerRef)))
    (:B
      (Pawn|Possess (Variables|Default|GetSleepingPawn)))))

(fn ConstructionScript)

(fn TitleScreen
  (Viewport|RemoveAllWidgets)
  (bind _returnvalue (UserInterface|CreateWidget "/Game/Blueprints/Widgets/Menu/Widget_Title.Widget_Title_C"))
  (UserInterface|Viewport|AddtoViewport _returnvalue 0)
  (Class|PlayerControllerBase|SetMouseState false))

(fn MainGame
  (Viewport|RemoveAllWidgets)
  (bind _returnvalue (UserInterface|CreateWidget "/Game/Blueprints/Widgets/Widget_MainUI.Widget_MainUI_C" self))
  (UserInterface|Viewport|AddtoViewport _returnvalue 0)
  (Variables|Default|SetMainUI _returnvalue)
  (Game|Player|SetViewTargetwithBlend (Game|GetPlayerController 0) (Pawn|GetControlledPawn) 0.0 "VTBlend_Linear" 1.0 false)
  (Class|PlayerControllerBase|SetMouseState true))

(fn GetPlayerRef
  (bind _returnvalue (Actor|GetActorOfClass "/Game/Blueprints/Player/BP_Player.BP_Player_C"))
  (Variables|Default|SetPlayerRef _returnvalue)
  (bind _returnvalue_2 (Actor|GetActorOfClass "/Game/Blueprints/Player/BP_PlayerSleeping.BP_PlayerSleeping_C"))
  (Variables|Default|SetSleepingPawn _returnvalue_2))
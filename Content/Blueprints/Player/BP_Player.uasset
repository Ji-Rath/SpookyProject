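; BP_Player is the player pawn Blueprint, routing input actions to interaction, physics grab and push, item dropping, inventory toggle and the pause menu.
; Interact component updates drive custom-depth highlighting of the focused pickupable's static mesh, clearing the previous one.
; The construction script assigns its inventory and equip components to inherited-style references.
; SPUD handles quick save and load, with overrides that keep transform and velocity restore enabled.
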(event Custom|HighlightPickupable
  (params (bInteractable :type Boolean) (Interactable :type Interactable%20Component%20Object%20Reference))
  (Utilities|Casting|CastToPickupableComponent Interactable
    (:then
      (Utilities|IsValid Interactable
        (:Is%20Valid
          (Variables|Default|GetInteractable
            (:then
              (Rendering|SetRenderCustomDepth (Actor|GetComponentbyClass (Variables|Default|GetInteractable) "/Script/Engine.StaticMeshComponent") false))
            (:else
              _))
          (Variables|Default|SetInteractable (Components|GetOwner Interactable))
          (Rendering|SetRenderCustomDepth (Actor|GetComponentbyClass (Variables|Default|GetInteractable) "/Script/Engine.StaticMeshComponent") true))
        (:Is%20Not%20Valid
          (Utilities|IsValid (Variables|Default|GetInteractable) :!label _label
            (:Is%20Valid
              (Rendering|SetRenderCustomDepth (Actor|GetComponentbyClass (Variables|Default|GetInteractable) "/Script/Engine.StaticMeshComponent") false)
              (Variables|Default|SetInteractable 0))))))
    (:CastFailed
      (goto _label))))

(event EventBeginPlay
  (|CallParentFunction)
  (EventDispatchers|AssignOnUpdateInteract (Variables|Default|GetBPC_PlayerInteractComponent) (delegate Custom|HighlightPickupable)))

(event Input|ActionEvents|InputActionInteract
  (params (Key :type Key%20Structure :default "None"))
  (:Pressed
    (Class|PlayerInteractComponent|Interact (Variables|Default|GetBPC_PlayerInteractComponent))))

(event Input|ActionEvents|InputActionGrab
  (params (Key :type Key%20Structure :default "None"))
  (:Pressed
    (Class|PhysicsGrabComponent|PhysicsInteract (Variables|Default|GetPhysicsGrab)))
  (:Released
    (Class|PhysicsGrabComponent|ReleaseComponent (Variables|Default|GetPhysicsGrab))))

(event Input|ActionEvents|InputActionPush
  (params (Key :type Key%20Structure :default "None"))
  (:Pressed
    (Class|PhysicsGrabComponent|PushGrabbedComponent (Variables|Default|GetPhysicsGrab))))

(event Input|ActionEvents|InputActionDropItem
  (params (Key :type Key%20Structure :default "None"))
  (:Pressed
    (Class|PlayerEquipComponent|DropEquippedItem (Variables|Default|GetPlayerEquip))))

(event Input|ActionEvents|InputActionEscape
  (params (Key :type Key%20Structure :default "None"))
  (:Pressed
    (bind _returnvalue (UserInterface|CreateWidget "/Game/Blueprints/Widgets/Menu/Widget_Pause.Widget_Pause_C" (CallFunction|GetPlayerController)))
    (UserInterface|Viewport|AddtoPlayerScreen _returnvalue)))

(event Input|ActionEvents|InputActionQuickSave
  (params (Key :type Key%20Structure :default "None"))
  (:Pressed
    (Class|SpudSubsystem|QuickSaveGame (Subsystems|GetSpudSubsystem) "House" true 0)))

(event Input|ActionEvents|InputActionQuickLoad
  (params (Key :type Key%20Structure :default "None"))
  (:Pressed
    (Class|SpudSubsystem|QuickLoadGame (Subsystems|GetSpudSubsystem))))

(event Input|ActionEvents|InputActionInventory
  (params (Key :type Key%20Structure :default "None"))
  (:Pressed
    (bind _asbp_player_controller (Utilities|Casting|CastToBP_PlayerController (Pawn|GetController)))
    (Default|ToggleInventory (Variables|/Game/Blueprints/Player/BP_PlayerController.BP_PlayerController_C|GetHUD _asbp_player_controller))))

(fn ConstructionScript
  (|CallParentFunction)
  (Variables|Default|SetInventoryComp (Variables|Default|GetBP_Inventory))
  (Variables|Default|SetEquipComp (Variables|Default|GetPlayerEquip)))

(fn ShouldSkipRestoreVelocity
  (return false))

(fn ShouldSkipRestoreTransform
  (return false))

(fn GetSpudRespawnMode
  (return "Default"))

(fn GetPlayerController
  (bind _asplayer_controller (Utilities|Casting|CastToPlayerController (Pawn|GetController)))
  (return _asplayer_controller))
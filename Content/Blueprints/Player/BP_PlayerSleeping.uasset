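; BP_PlayerSleeping is the player's sleeping state, in which the player can look around and try to wake up.
; Look axes feed controller pitch and yaw.
; Pressing Interact while CanWakeup is set casts through BP_PlayerController to its MainUI widget and plays the blink animation.
; The file itself performs no wake-up or pawn switch beyond triggering that animation.
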(event Input|ActionEvents|InputActionInteract
  (params (Key :type Key%20Structure :default "None"))
  (:Pressed
    (if (Variables|Default|GetbCanWakeup)
      (bind _asbp_player_controller (Utilities|Casting|CastToBP_PlayerController (Game|GetPlayerController 0)))
      (bind _aswidget_main_ui (Utilities|Casting|CastToWidget_MainUI (Variables|/Script/SpookyGame.PlayerControllerBase|GetMainUI _asbp_player_controller)))
      (Default|PlayBlinkAnim _aswidget_main_ui))))

(event Input|AxisEvents|InputAxisLookUp
  (params (AxisValue :type Float%20%28single-precision%29))
  (Pawn|Input|AddControllerPitchInput AxisValue))

(event Input|AxisEvents|InputAxisLookRight
  (params (AxisValue :type Float%20%28single-precision%29))
  (Pawn|Input|AddControllerYawInput AxisValue))

(fn ConstructionScript)
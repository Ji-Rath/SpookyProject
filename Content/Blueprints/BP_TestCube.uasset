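; BP_TestCube is a test actor for experimenting with shadow projection from a light.
; ProjectShadowTest offsets each point in an array by the actor's location and line-traces 500 units from it, directly away from LightActor.
; The traces draw for one frame as debug, and their results are unused.
; Tick is empty; the shadow test call and a LightSense light-level print are both disconnected.
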(event EventBeginPlay)

(event Collision|EventActorBeginOverlap
  (params (OtherActor :type Actor%20Object%20Reference)))

(event EventTick
  (params (DeltaSeconds :type Float%20%28single-precision%29)))

(fn ConstructionScript)

(fn ProjectShadowTest
  (for _array_element (Variables|Default|GetNewVar_0)
    (Collision|LineTraceByChannel (+ _array_element (Transformation|GetActorLocation)) (+ (+ _array_element (Transformation|GetActorLocation)) (* (Math|Vector|GetForwardVector (Math|Rotator|FindLookatRotation (Transformation|GetActorLocation (Variables|Default|GetLightActor)) (+ _array_element (Transformation|GetActorLocation)))) 5e+02)) "TraceTypeQuery1" false 0 "ForOneFrame")))
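; BP_Particles is an actor Blueprint that drives a Niagara particle effect tied to a referenced light actor.
; It writes the light actor's location to the system's LightPos parameter during construction and on every Tick, keeping the effect updated as the light moves.
; The Construction Script also passes the Direction variable into Niagara.
; OnInteract resets the particle system.
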(event EventOnInteract
  (params (Interactor :type Actor%20Object%20Reference))
  (Niagara|ResetSystem (Variables|Default|GetNiagaraParticle)))

(event EventTick
  (params (DeltaSeconds :type Float%20%28single-precision%29))
  (CallFunction|UpdateFollowPos))

(fn ConstructionScript
  (CallFunction|UpdateFollowPos)
  (Niagara|SetNiagaraVariable(Float) (Variables|Default|GetNiagaraParticle) "Direction" (Variables|Default|GetDirection)))

(fn UpdateFollowPos
  (Niagara|SetNiagaraVariable(Vector3) (Variables|Default|GetNiagaraParticle) "LightPos" (Transformation|GetActorLocation (Variables|Default|GetLightActor))))